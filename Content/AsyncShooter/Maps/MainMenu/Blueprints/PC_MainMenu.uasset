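; Main menu player controller that shows the WB_MainMenu widget with a mouse cursor and handles menu navigation input.
; Steam Input digital presses are injected as Enhanced Input menu actions under MC_Menu, so they share one path with other bound inputs.
; Each action's Started event calls a matching OnMenu dispatcher for directions, select and cancel.
; Helpers fetch connected controllers and action glyphs, while analog, just-pressed and release handlers do nothing.
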(event `self.ReceiveBeginPlay`
  (bind _returnvalue (`GameplayStatics.GetPlayerController` 0))
  (add `self.OnSteamDigitalInputJustReleased` (`|CreateDelegate` :!event `DigitalInputJustReleased`))
  (add `self.OnSteamDigitalInputPressed` (`|CreateDelegate` :!event `DigitalInputPressed`))
  (add `self.OnSteamDigitalInputReleased` (`|CreateDelegate` :!event `DigitalInputReleased`))
  (add `self.OnSteamDigitalInputJustPressed` (`|CreateDelegate` :!event `DigitalInputJustPressed`))
  (add `self.OnSteamAnalogInput` (`|CreateDelegate` :!event `AnalogInput`))
  (message `EnhancedInputSubsystemInterface.AddMappingContext` (pcsubsystem `EnhancedInputLocalPlayerSubsystem` _returnvalue) "/Game/AsyncShooter/Blueprints/Menu/Input/MC_Menu.MC_Menu" 0 (struct))
  (bind _returnvalue_2 (`|CreateWidget` "/Game/AsyncShooter/Maps/MainMenu/Blueprints/WB_MainMenu.WB_MainMenu_C" _returnvalue))
  (`WidgetBlueprintLibrary.SetInputMode_GameAndUIEx` _returnvalue _returnvalue_2 "LockAlways" false true)
  (`UserWidget.AddToViewport` _returnvalue_2 0)
  (set `self.bShowMouseCursor` true))

(event `EnhancedInput|/Game/AsyncShooter/Blueprints/Menu/Input/A_MenuUp`
  (params (ActionValue :type Boolean) (ElapsedSeconds :type "Float (double-precision)") (TriggeredSeconds :type "Float (double-precision)") (InputAction :type "InputAction Object Reference" :default "/Game/AsyncShooter/Blueprints/Menu/Input/A_MenuUp.A_MenuUp"))
  (:`Started`
    (if (not false)
      (`self.OnMenuUp`))))

(event `EnhancedInput|/Game/AsyncShooter/Blueprints/Menu/Input/A_MenuDown`
  (params (ActionValue :type Boolean) (ElapsedSeconds :type "Float (double-precision)") (TriggeredSeconds :type "Float (double-precision)") (InputAction :type "InputAction Object Reference" :default "/Game/AsyncShooter/Blueprints/Menu/Input/A_MenuDown.A_MenuDown"))
  (:`Started`
    (if (not false)
      (`self.OnMenuDown`))))

(event `EnhancedInput|/Game/AsyncShooter/Blueprints/Menu/Input/A_MenuLeft`
  (params (ActionValue :type Boolean) (ElapsedSeconds :type "Float (double-precision)") (TriggeredSeconds :type "Float (double-precision)") (InputAction :type "InputAction Object Reference" :default "/Game/AsyncShooter/Blueprints/Menu/Input/A_MenuLeft.A_MenuLeft"))
  (:`Started`
    (if (not false)
      (`self.OnMenuLeft`))))

(event `EnhancedInput|/Game/AsyncShooter/Blueprints/Menu/Input/A_MenuRight`
  (params (ActionValue :type Boolean) (ElapsedSeconds :type "Float (double-precision)") (TriggeredSeconds :type "Float (double-precision)") (InputAction :type "InputAction Object Reference" :default "/Game/AsyncShooter/Blueprints/Menu/Input/A_MenuRight.A_MenuRight"))
  (:`Started`
    (if (not false)
      (`self.OnMenuRight`))))

(event `EnhancedInput|/Game/AsyncShooter/Blueprints/Menu/Input/A_MenuCancel`
  (params (ActionValue :type Boolean) (ElapsedSeconds :type "Float (double-precision)") (TriggeredSeconds :type "Float (double-precision)") (InputAction :type "InputAction Object Reference" :default "/Game/AsyncShooter/Blueprints/Menu/Input/A_MenuCancel.A_MenuCancel"))
  (:`Started`
    (if (not false)
      (`self.OnMenuCancel`))))

(event `EnhancedInput|/Game/AsyncShooter/Blueprints/Menu/Input/A_MenuSelect`
  (params (ActionValue :type Boolean) (ElapsedSeconds :type "Float (double-precision)") (TriggeredSeconds :type "Float (double-precision)") (InputAction :type "InputAction Object Reference" :default "/Game/AsyncShooter/Blueprints/Menu/Input/A_MenuSelect.A_MenuSelect"))
  (:`Started`
    (if (not false)
      (`self.OnMenuSelect`))))

(fn `AnalogInput`
  (params (InputAction :type String) (State :type "Vector2D Structure") (InputSourceMode :type "ECInputSourceMode Enum" :default "None")))

(fn `DigitalInputJustPressed`
  (params (InputAction :type String)))

(fn `DigitalInputJustReleased`
  (params (InputAction :type String))
  (switch `string` InputAction))

(fn `DigitalInputPressed`
  (params (InputAction :type String) (ElapsedSeconds :type "Float (double-precision)"))
  (bind _returnvalue (`EnhancedInputLibrary.MakeInputActionValueOfType` 1.0 1.0 1.0 "Boolean"))
  (bind _returnvalue_2 (pcsubsystem `EnhancedInputLocalPlayerSubsystem` self))
  (switch `string` InputAction
    (:`menu_up`
      (`EnhancedInputSubsystemInterface.InjectInputForAction` :`self` _returnvalue_2 :`Action` "/Game/AsyncShooter/Blueprints/Menu/Input/A_MenuUp.A_MenuUp" :`RawValue` _returnvalue))
    (:`menu_down`
      (`EnhancedInputSubsystemInterface.InjectInputForAction` :`self` _returnvalue_2 :`Action` "/Game/AsyncShooter/Blueprints/Menu/Input/A_MenuDown.A_MenuDown" :`RawValue` _returnvalue))
    (:`menu_left`
      (`EnhancedInputSubsystemInterface.InjectInputForAction` :`self` _returnvalue_2 :`Action` "/Game/AsyncShooter/Blueprints/Menu/Input/A_MenuLeft.A_MenuLeft" :`RawValue` _returnvalue))
    (:`menu_right`
      (`EnhancedInputSubsystemInterface.InjectInputForAction` :`self` _returnvalue_2 :`Action` "/Game/AsyncShooter/Blueprints/Menu/Input/A_MenuRight.A_MenuRight" :`RawValue` _returnvalue))
    (:`menu_select`
      (`EnhancedInputSubsystemInterface.InjectInputForAction` :`self` _returnvalue_2 :`Action` "/Game/AsyncShooter/Blueprints/Menu/Input/A_MenuSelect.A_MenuSelect" :`RawValue` _returnvalue))
    (:`menu_cancel`
      (`EnhancedInputSubsystemInterface.InjectInputForAction` :`self` _returnvalue_2 :`Action` "/Game/AsyncShooter/Blueprints/Menu/Input/A_MenuCancel.A_MenuCancel" :`RawValue` _returnvalue))))

(fn `DigitalInputReleased`
  (params (InputAction :type String) (ElapsedSeconds :type "Float (single-precision)"))
  (switch `string` InputAction))

(fn `GetControllers`
  (bind _returnvalue (`FL_SteamInput.GetConnectedControllers`))
  (set `self.Controllers` _returnvalue))

(fn `GetGlyphPathForAction`
  (params (Action :type String))
  (returns (GlyphPath :type String))
  (bind _returnvalue (`self.GetCurrentGlyphForAction` Action))
  (return _returnvalue))

(fn `UserConstructionScript`)