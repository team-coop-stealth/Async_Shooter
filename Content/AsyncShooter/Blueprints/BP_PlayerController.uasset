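; Player controller that lets the player choose between the Agent and Hacker roles in a stealth game.
; On BeginPlay it shows the SelectRoles widget with the menu input context and mouse cursor, binding each choice to a creation event.
; Each choice spawns BP_Ninja or BP_Hacker at the origin through Server-named events, possesses it, then initialises the matching BP_StealthHUD view.
; The cursor is hidden only for the Agent.
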(event `self.ReceiveBeginPlay`
  (`self.SelectRoles`))

(event `SelectRoles`
  (bind _returnvalue (`|CreateWidget` "/Game/AsyncShooter/Blueprints/UI/SelectRoles.SelectRoles_C" (`GameplayStatics.GetPlayerController` 0)))
  (`UserWidget.AddToViewport` _returnvalue 0)
  (add `/Game/AsyncShooter/Blueprints/UI/SelectRoles.AddAgent` _returnvalue (delegate `CreateAgent`))
  (add `/Game/AsyncShooter/Blueprints/UI/SelectRoles.AddHacker` _returnvalue (delegate `CreateHacker_Event`))
  (`EnhancedInputSubsystemInterface.AddMappingContext` (pcsubsystem `EnhancedInputLocalPlayerSubsystem` (`GameplayStatics.GetPlayerController` 0)) "/Game/AsyncShooter/Blueprints/Menu/Input/MC_Menu.MC_Menu" 0 (struct))
  (set `self.bShowMouseCursor` true))

(event `CreateHacker_Event`
  (`self.CreateHackerServer`)
  (bind _asbp_stealth_hud (cast `/Game/AsyncShooter/Blueprints/BP_StealthHUD` (`self.GetHUD`)))
  (`/Game/AsyncShooter/Blueprints/BP_StealthHUD.InitHackerHUD` _asbp_stealth_hud self))

(event `CreateHackerServer`
  (bind _returnvalue (`|SpawnActorFromClass` "/Game/AsyncShooter/Blueprints/Hacker/BP_Hacker.BP_Hacker_C" (`KismetMathLibrary.MakeTransform` (0.0 0.0 0.0)) "AdjustIfPossibleButAlwaysSpawn" "MultiplyWithRoot" null null))
  (`self.PossessPlayerAsClient` self _returnvalue))

(event `CreateAgent`
  (`self.CreateAgentServer`)
  (bind _asbp_stealth_hud (cast `/Game/AsyncShooter/Blueprints/BP_StealthHUD` (`self.GetHUD`)))
  (`/Game/AsyncShooter/Blueprints/BP_StealthHUD.InitAgentHUD` _asbp_stealth_hud self)
  (set `self.bShowMouseCursor` false))

(event `CreateAgentServer`
  (bind _returnvalue (`|SpawnActorFromClass` "/Game/AsyncShooter/Blueprints/Ninja/BP_Ninja.BP_Ninja_C" (`KismetMathLibrary.MakeTransform` (0.0 0.0 0.0)) "AdjustIfPossibleButAlwaysSpawn" "MultiplyWithRoot" null null))
  (`self.PossessPlayerAsClient` self _returnvalue))

(event `PossessPlayerAsClient`
  (params (Target :type "PlayerController Object Reference") (`In Pawn` :type "Pawn Object Reference"))
  (`self.Possess` `In Pawn`))

(fn `NewFunction`)

(fn `UserConstructionScript`)