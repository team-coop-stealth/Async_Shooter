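; BP_CallGadget is a hacker gadget built around a loudspeaker that makes noise for AI hearing when activated.
; At BeginPlay it binds Activate to the click of its WB_ActivateButton widget.
; Activate reports a noise event at the speaker's location offset by CallLocation and prints a debug string.
; Each tick, on authority only, the button's visibility follows whether the speaker mesh was recently rendered.
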(event `self.ReceiveBeginPlay`
  (bind _aswb_activate_button (cast `/Game/AsyncShooter/Blueprints/HackerGadgets/WB_ActivateButton` (`WidgetComponent.GetWidget` (`self.ActivateButton`))))
  (add `/Game/AsyncShooter/Blueprints/HackerGadgets/WB_ActivateButton.ButtonClicked` _aswb_activate_button (delegate `Activate`)))

(event `Activate`
  (`AISense_Hearing.ReportNoiseEvent` (+ (`self.CallLocation`) (`SceneComponent.K2_GetComponentLocation` (`self.Loudspeaker_03_Loudspeaker_033`))) 2.0 self)
  (`KismetSystemLibrary.PrintString` "Boom"))

(event `self.ReceiveTick`
  (params (DeltaSeconds :type "Float (single-precision)"))
  (`/Engine/EditorBlueprintResources/ActorMacros.Switch Has Authority`
    (:`Authority`
      (`SceneComponent.SetVisibility` (`self.ActivateButton`) (`PrimitiveComponent.WasRecentlyRendered` (`self.Loudspeaker_03_Loudspeaker_033`) 0.2) false))))

(fn `UserConstructionScript`)