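; BP_Hacker is the possessable hacker character in AsyncShooter, which hovers directly above the ninja.
; On possession it shows the mouse cursor for the player controller.
; Every tick it looks up all BP_Ninja actors and moves itself to the first one's location, raised by DistanceFromNinja, without sweeping or smoothing.
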(event `self.ReceivePossessed`
  (params (NewController :type "Controller Object Reference"))
  (bind _asplayer_controller (cast `PlayerController` NewController))
  (set `PlayerController.bShowMouseCursor` true _asplayer_controller))

(event `self.ReceiveTick`
  (params (DeltaSeconds :type "Float (single-precision)"))
  (bind _outactors (`GameplayStatics.GetAllActorsOfClass` "/Game/AsyncShooter/Blueprints/Ninja/BP_Ninja.BP_Ninja_C"))
  (`self.K2_SetActorLocation` (`KismetMathLibrary.MakeVector` (.x (`self.K2_GetActorLocation` (`|GetArrayItem` _outactors))) (.y (`self.K2_GetActorLocation` (`|GetArrayItem` _outactors))) (+ (`self.DistanceFromNinja`) (.z (`self.K2_GetActorLocation` (`|GetArrayItem` _outactors)))))))

(fn `UserConstructionScript`)